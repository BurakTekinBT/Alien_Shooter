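; Bullet is a projectile actor that flies straight forward and damages Enemy actors it hits.
; Each tick moves it along its forward vector at MoveSpeed without sweeping and destroys it once LifeTime has passed since BeginPlay, measured in real seconds.
; An overlap with an Enemy calls TakeDamage with a hard-coded amount and destroys the bullet; other actors are ignored.
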(event `self.ReceiveBeginPlay`
  (set `self.StartTime` (`GameplayStatics.GetRealTimeSeconds`)))

(event `self.ReceiveTick`
  (params (DeltaSeconds :type "Float (single-precision)"))
  (`self.K2_AddActorWorldOffset` (* (`self.GetActorForwardVector`) (* DeltaSeconds (`self.MoveSpeed`))))
  (if (>= (`GameplayStatics.GetRealTimeSeconds`) (+ (`self.StartTime`) (`self.LifeTime`)))
    (`self.K2_DestroyActor`)))

(event `self.ReceiveActorBeginOverlap`
  (params (OtherActor :type "Actor Object Reference"))
  (bind _asenemy (cast `/Game/Blueprints/Enemy` OtherActor))
  (`/Game/Blueprints/Enemy.TakeDamage` _asenemy 15)
  (`self.K2_DestroyActor`))

(fn `UserConstructionScript`)